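; Two-statue rotation puzzle where the player turns angel statues to reveal what lies behind tagged walls.
; Each statue's proximity trigger enables input and opens a gate, letting E play a timeline that yaws it by Angle, with input locked during the turn.
; Activation triggers overlapping BP_Activepuzzle flag each statue active.
; A looping timer polls both flags and, when both are set, hides StaticMeshActors tagged "Hide" without changing their collision.
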(event OnComponentEndOverlap(Trigger1)
  (params (OverlappedComponent :type Primitive%20Component%20Object%20Reference) (OtherActor :type Actor%20Object%20Reference) (OtherComp :type Primitive%20Component%20Object%20Reference) (OtherBodyIndex :type Integer))
  (bind _returnvalue (Game|GetPlayerController 0))
  (Utilities|Casting|CastToBP_FirstPersonCharacter OtherActor)
  (Input|DisableInput (Game|GetPlayerController 0))
  (Utilities|FlowControl|Gate true) ; enters at Close
)

(event OnComponentBeginOverlap(TriggerActivation1)
  (params (OverlappedComponent :type Primitive%20Component%20Object%20Reference) (OtherActor :type Actor%20Object%20Reference) (OtherComp :type Primitive%20Component%20Object%20Reference) (OtherBodyIndex :type Integer) (bFromSweep :type Boolean) (SweepResult :type Hit%20Result%20Structure%20%28by%20ref%29))
  (Utilities|Casting|CastToBP_Activepuzzle OtherActor)
  (Variables|Default|SetStatue2Active true))

(event OnComponentEndOverlap(TriggerActivation1)
  (params (OverlappedComponent :type Primitive%20Component%20Object%20Reference) (OtherActor :type Actor%20Object%20Reference) (OtherComp :type Primitive%20Component%20Object%20Reference) (OtherBodyIndex :type Integer))
  (Utilities|Casting|CastToBP_Activepuzzle OtherActor)
  (Variables|Default|SetStatue2Active false))

(event OnComponentBeginOverlap(TriggerActivation)
  (params (OverlappedComponent :type Primitive%20Component%20Object%20Reference) (OtherActor :type Actor%20Object%20Reference) (OtherComp :type Primitive%20Component%20Object%20Reference) (OtherBodyIndex :type Integer) (bFromSweep :type Boolean) (SweepResult :type Hit%20Result%20Structure%20%28by%20ref%29))
  (Utilities|Casting|CastToBP_Activepuzzle OtherActor)
  (Variables|Default|SetStatue1Active true))

(event OnComponentEndOverlap(TriggerActivation)
  (params (OverlappedComponent :type Primitive%20Component%20Object%20Reference) (OtherActor :type Actor%20Object%20Reference) (OtherComp :type Primitive%20Component%20Object%20Reference) (OtherBodyIndex :type Integer))
  (Utilities|Casting|CastToBP_Activepuzzle OtherActor)
  (Variables|Default|SetStatue1Active false))

(event OnComponentBeginOverlap(Trigger)
  (params (OverlappedComponent :type Primitive%20Component%20Object%20Reference) (OtherActor :type Actor%20Object%20Reference) (OtherComp :type Primitive%20Component%20Object%20Reference) (OtherBodyIndex :type Integer) (bFromSweep :type Boolean) (SweepResult :type Hit%20Result%20Structure%20%28by%20ref%29))
  (bind _returnvalue (Game|GetPlayerController 0))
  (Utilities|Casting|CastToBP_FirstPersonCharacter OtherActor)
  (Input|EnableInput (Game|GetPlayerController 0))
  (Utilities|FlowControl|Gate true) ; enters at Open
)

(event OnComponentEndOverlap(Trigger)
  (params (OverlappedComponent :type Primitive%20Component%20Object%20Reference) (OtherActor :type Actor%20Object%20Reference) (OtherComp :type Primitive%20Component%20Object%20Reference) (OtherBodyIndex :type Integer))
  (bind _returnvalue (Game|GetPlayerController 0))
  (Utilities|Casting|CastToBP_FirstPersonCharacter OtherActor)
  (Input|DisableInput (Game|GetPlayerController 0))
  (Utilities|FlowControl|Gate true) ; enters at Close
)

(event OnComponentBeginOverlap(Trigger1)
  (params (OverlappedComponent :type Primitive%20Component%20Object%20Reference) (OtherActor :type Actor%20Object%20Reference) (OtherComp :type Primitive%20Component%20Object%20Reference) (OtherBodyIndex :type Integer) (bFromSweep :type Boolean) (SweepResult :type Hit%20Result%20Structure%20%28by%20ref%29))
  (bind _returnvalue (Game|GetPlayerController 0))
  (Utilities|Casting|CastToBP_FirstPersonCharacter OtherActor)
  (Input|EnableInput (Game|GetPlayerController 0))
  (Utilities|FlowControl|Gate true) ; enters at Open
)

(event Custom|PuzzleDone
  (if (and (Variables|Default|GetStatue1Active) (Variables|Default|GetStatue2Active))
    (CallFunction|HideWALS)
    (Actor|GetAllActorsOfClasswithTag "/Script/Engine.StaticMeshActor" "Hide")))

(event Custom|HideWALS
  (Actor|GetAllActorsOfClasswithTag "/Script/Engine.StaticMeshActor" "Hide")
  (for _array_element 0
    (Rendering|SetActorHiddenInGame _array_element true)))

(event EventBeginPlay
  (Utilities|FlowControl|Sequence
    (:then_0
      (Variables|Default|SetCurrentRotationE1 (Transformation|GetWorldRotation (Variables|Default|Getangel_1)))
      (Variables|Default|SetCurrentRotationE2 (Transformation|GetWorldRotation (Variables|Default|Getangel_2))))
    (:then_1
      (Utilities|Time|SetTimerbyFunctionName 0 "PuzzleDone" 0.25 true))))

(event Input|ActionEvents|InputActionE
  (params (Key :type Key%20Structure :default "None"))
  (bind _returnvalue (Game|GetPlayerController 0))
  (:Pressed
    (Utilities|FlowControl|Gate true
      (:Exit
        (Input|DisableInput _returnvalue)
        (bind _giro (Timeline|Timeline PlayFromStart)
          (:Update
            (Transformation|SetRelativeRotation (Variables|Default|Getangel_2) (Math|Rotator|Lerp(Rotator) (Variables|Default|GetCurrentRotationE2) (Math|Rotator|MakeRotator (.Roll (Math|Rotator|BreakRotator (Variables|Default|GetCurrentRotationE2))) (.Pitch (Math|Rotator|BreakRotator (Variables|Default|GetCurrentRotationE2))) (+ (.Yaw (Math|Rotator|BreakRotator (Variables|Default|GetCurrentRotationE2))) (Variables|Default|GetAngle))) _giro) false false))
          (:Finished
            (Variables|Default|SetCurrentRotationE2 (Math|Rotator|Lerp(Rotator) (Variables|Default|GetCurrentRotationE2) (Math|Rotator|MakeRotator (.Roll (Math|Rotator|BreakRotator (Variables|Default|GetCurrentRotationE2))) (.Pitch (Math|Rotator|BreakRotator (Variables|Default|GetCurrentRotationE2))) (+ (.Yaw (Math|Rotator|BreakRotator (Variables|Default|GetCurrentRotationE2))) (Variables|Default|GetAngle))) _giro))
            (Input|EnableInput _returnvalue)))))))

(event Input|ActionEvents|InputActionE
  (params (Key :type Key%20Structure :default "None"))
  (bind _returnvalue (Game|GetPlayerController 0))
  (:Pressed
    (Utilities|FlowControl|Gate true
      (:Exit
        (Input|DisableInput _returnvalue)
        (bind _giro (Timeline|TimelineEstatua1 PlayFromStart)
          (:Update
            (Transformation|SetRelativeRotation (Variables|Default|Getangel_1) (Math|Rotator|Lerp(Rotator) (Variables|Default|GetCurrentRotationE1) (Math|Rotator|MakeRotator (.Roll (Math|Rotator|BreakRotator (Variables|Default|GetCurrentRotationE1))) (.Pitch (Math|Rotator|BreakRotator (Variables|Default|GetCurrentRotationE1))) (+ (.Yaw (Math|Rotator|BreakRotator (Variables|Default|GetCurrentRotationE1))) (Variables|Default|GetAngle))) _giro) false false))
          (:Finished
            (Variables|Default|SetCurrentRotationE1 (Math|Rotator|Lerp(Rotator) (Variables|Default|GetCurrentRotationE1) (Math|Rotator|MakeRotator (.Roll (Math|Rotator|BreakRotator (Variables|Default|GetCurrentRotationE1))) (.Pitch (Math|Rotator|BreakRotator (Variables|Default|GetCurrentRotationE1))) (+ (.Yaw (Math|Rotator|BreakRotator (Variables|Default|GetCurrentRotationE1))) (Variables|Default|GetAngle))) _giro))
            (Input|EnableInput _returnvalue)))))))

(fn ConstructionScript)